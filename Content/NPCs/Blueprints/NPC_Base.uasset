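; Base NPC that shows its name, opens dialogue on interaction and can patrol or turn between destination actors.
; Patrol loops AI moves through the destinations, while optional rotation loops a timeline yaw lerp toward each, both pausing between targets.
; Pawn sensing halts movement and can interrupt with dialogue; later sightings without an open dialogue restore walking and re-arm interruption after a delay.
; NPCs without a vision cone destroy their sensing and line-of-sight visual components.
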(event OnSeePawn(PawnSensing)
  (params (Pawn :type Pawn%20Object%20Reference))
  (bind _ac_dialogue_test (Variables|Default|GetAC_Dialogue_Test))
  (bind _dialoguewidget (Variables|/Game/Dialogue/Core/AC_Dialogue_Base.AC_Dialogue_Base_C|GetDialogueWidget _ac_dialogue_test))
  (bind _returnvalue (Utilities|IsValid _dialoguewidget))
  (Pawn|Components|CharacterMovement|DisableMovement (Variables|Character|GetCharacterMovement))
  (if (Variables|Default|GetCanInterrupt)
    (if (not _returnvalue)
      (Variables|Default|SetCanInterrupt false)
      (Variables|Default|SetInteractInstigator self)
      (Default|OpenConversation _ac_dialogue_test))
    (elif (not _returnvalue)
      (Pawn|Components|CharacterMovement|SetMovementMode (Variables|Character|GetCharacterMovement) "MOVE_Walking" 0)
      (Utilities|FlowControl|Delay 3.0)
      (Variables|Default|SetCanInterrupt true))))

(event Custom|Patrol
  (if (Variables|Default|GetCanPatrol)
    (AI|AIMoveTo self "0, 0, 0" (Utilities|Array|Get(acopy) (Variables|Default|GetDestinations) (Variables|Default|GetTarget)) 5.0 true :!label _label
      (:OnSuccess
        (if (== (+ (Variables|Default|GetTarget) 1) (Utilities|Array|Length (Variables|Default|GetDestinations)))
          (Variables|Default|SetTarget 0)
          (else
            (Variables|Default|SetTarget (+ (Variables|Default|GetTarget) 1))))
        (Utilities|FlowControl|Delay (Variables|Default|GetWait))
        (goto _label)))))

(event Custom|StartRotate
  (Variables|Default|SetCurrentRotation (Transformation|GetActorRotation) :!label _label)
  (bind _alpha (Timeline|Timeline PlayFromStart)
    (:Update
      (Transformation|SetActorRotation (Math|Rotator|Lerp(Rotator) (Variables|Default|GetCurrentRotation) (Math|Rotator|MakeRotator 0.0 0.0 (.yaw (Math|Rotator|FindLookatRotation (Transformation|GetActorLocation) (Transformation|GetActorLocation (Utilities|Array|Get(acopy) (Variables|Default|GetDestinations) (Variables|Default|GetTarget)))))) _alpha)))
    (:Finished
      (if (== (+ (Variables|Default|GetTarget) 1) (Utilities|Array|Length (Variables|Default|GetDestinations)))
        (Variables|Default|SetTarget 0)
        (else
          (Variables|Default|SetTarget (+ (Variables|Default|GetTarget) 1))))
      (Utilities|FlowControl|Delay (Variables|Default|GetWait))
      (goto _label))))

(event Custom|EnableVisionCone
  (if (not (Variables|Default|GetHasVisionCone))
    (Components|DestroyComponent (Variables|Default|GetPawnSensing))
    (Components|DestroyComponent (Variables|Default|GetLOSVisual))))

(event EventTick
  (params (DeltaSeconds :type Float%20%28single-precision%29)))

(event EventBeginPlay
  (CallFunction|Patrol)
  (CallFunction|EnableVisionCone)
  (if (Variables|Default|GetRotates)
    (CallFunction|StartRotate)))

(event EventInteract
  (params (Instigator :type Actor%20Object%20Reference))
  (Variables|Default|SetInteractInstigator Instigator)
  (Default|OpenConversation (Variables|Default|GetAC_Dialogue_Test)))

(fn ConstructionScript
  (Rendering|Components|TextRender|SetText (Variables|Default|GetTxt_CharacterName) (Variables|Default|GetCharacterName)))