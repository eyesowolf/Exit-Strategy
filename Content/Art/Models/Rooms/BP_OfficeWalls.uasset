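; BP_OfficeWalls is an office room wall actor that can switch from a closed to an open layout.
; On BeginPlay it caches the first actor tagged OfficeDoor.
; OpenWalls sets an Open flag, shows static mesh components tagged Open and hides those tagged Closed, and hides that door actor and disables its collision.
; The switch is one-way, as no close function exists.
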(event EventBeginPlay
  (bind _outactors (Actor|GetAllActorswithTag "OfficeDoor"))
  (Variables|Default|SetOfficeDoor (Utilities|Array|Get(acopy) _outactors)))

(fn ConstructionScript)

(fn OpenWalls
  (bind _officedoor (Variables|Default|GetOfficeDoor))
  (Variables|Default|SetOpen true)
  (for _array_element (Actor|GetComponentsbyTag "/Script/Engine.StaticMeshComponent" "Open")
    (Rendering|SetVisibility _array_element true false))
  (Rendering|SetActorHiddenInGame _officedoor true)
  (Collision|SetActorEnableCollision _officedoor false)
  (for _array_element_2 (Actor|GetComponentsbyTag "/Script/Engine.StaticMeshComponent" "Closed")
    (Rendering|SetVisibility _array_element_2 false false)))