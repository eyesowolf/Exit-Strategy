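; Dialogue component for the office door keypad, presenting the player's musing about what is inside and which code to try.
; It overrides Dialogue as a tree switched on DialogueTreeIndex, with index 0 routing by HasCode2 to a branch with or without the Code2 option.
; AddDialogue nodes chain lines and choices until the conversation closes.
; Selecting the code has no effect yet, and the CodeOptions list-building is unwired.
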(fn Dialogue
  (|CallParentFunction)
  (switch int (Variables|Default|GetDialogueTreeIndex) :!label _label
    (:0
      (if (Variables|Default|GetHasCode2)
        (Variables|Default|SetDialogueTreeIndex 2)
        (goto _label)
        (else
          (Variables|Default|SetDialogueTreeIndex 1)
          (goto _label))))
    (:1
      (bind (_state _optionindex) (CallFunction|AddDialogue (Variables|Default|GetNPCName) "There's a keypad on this door. I wonder what's in there." (Utilities|Array|MakeArray "...")))
      (switch Utilities|FlowControl|Switch|SwitchonEnum_DialogueState _state
        (:NewEnumerator0
          (switch int _optionindex
            (:0
              (bind _state_2 (CallFunction|AddDialogue (Variables|Default|GetNPCName) "Can I think of a code to try?" (Utilities|Array|MakeArray "Not right now.")))
              (switch Utilities|FlowControl|Switch|SwitchonEnum_DialogueState _state_2
                (:NewEnumerator0
                  (CallFunction|SetDialogueTreeIndex)
                  (CallFunction|CloseConversation))))))))
    (:2
      (bind (_state_3 _optionindex_2) (CallFunction|AddDialogue (Variables|Default|GetNPCName) "There's a keypad on this door. I wonder what's in there." (Utilities|Array|MakeArray "...")))
      (switch Utilities|FlowControl|Switch|SwitchonEnum_DialogueState _state_3
        (:NewEnumerator0
          (switch int _optionindex_2
            (:0
              (bind (_state_4 _optionindex_3) (CallFunction|AddDialogue (Variables|Default|GetNPCName) "Can I think of a code to try?" (Utilities|Array|MakeArray "Not right now." (Variables|Default|GetCode2Text))))
              (switch Utilities|FlowControl|Switch|SwitchonEnum_DialogueState _state_4
                (:NewEnumerator0
                  (bind _state_5 (CallFunction|AddDialogue (Variables|Default|GetNPCName) "Can I think of a code to try?" (Utilities|Array|MakeArray "Not right now.")))
                  (switch Utilities|FlowControl|Switch|SwitchonEnum_DialogueState _state_5
                    (:NewEnumerator0
                      (CallFunction|CloseConversation))))
                (:NewEnumerator1
                  (if (== _optionindex_3 1)
                    _))))))))))

(fn ConversationOpened
  (return 0))