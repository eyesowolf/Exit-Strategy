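; Dialogue component for the Grandpa NPC, scripting party small talk and his offer to open a door in exchange for a cookie.
; The Dialogue function extends its parent and switches on DialogueTreeIndex, chaining AddDialogue prompts by state and chosen option.
; Branches update the index or close the conversation, and an inventory check for the Cookie re-enters the switch.
; The door-opening promise is only spoken text here, with no door logic.
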(event EventBeginPlay)

(fn Dialogue
  (|CallParentFunction)
  (switch int (Variables|Default|GetDialogueTreeIndex) :!label _label
    (:0
      (bind _state (CallFunction|AddDialogue (Variables|Default|GetNPCName) "Enjoying the party?" (Utilities|Array|MakeArray "It's great!" "About as much as ")))
      (switch Utilities|FlowControl|Switch|SwitchonEnum_DialogueState _state))
    (:1
      (bind (_state_2 _optionindex) (CallFunction|AddDialogue (Variables|Default|GetNPCName) "Enjoying the party?" (Utilities|Array|MakeArray "What do you think?" "Can you open that door for me?")))
      (switch Utilities|FlowControl|Switch|SwitchonEnum_DialogueState _state_2
        (:NewEnumerator0
          (switch int _optionindex
            (:0
              (bind _state_3 (CallFunction|AddDialogue (Variables|Default|GetNPCName) "Sounds like you're loving it!" (Utilities|Array|MakeArray "Ugh fiiiine.")))
              (switch Utilities|FlowControl|Switch|SwitchonEnum_DialogueState _state_3
                (:NewEnumerator0
                  (CallFunction|CloseConversation))))
            (:1
              (bind _state_4 (CallFunction|AddDialogue (Variables|Default|GetNPCName) "I'll open it if you get me a cookie from the snacks table." (Utilities|Array|MakeArray "Ugh fiiiine.")))
              (switch Utilities|FlowControl|Switch|SwitchonEnum_DialogueState _state_4
                (:NewEnumerator0
                  (CallFunction|SetDialogueTreeIndex 1)
                  (CallFunction|CloseConversation))))))))
    (:2
      (bind _hasitem (CallFunction|CheckPlayerItems "Cookie"))
      (if _hasitem
        (Variables|Default|SetDialogueTreeIndex 3)
        (goto _label)
        (else
          (CallFunction|SetDialogueTreeIndex 2)
          (goto _label))))
    (:3
      (bind _state_5 (CallFunction|AddDialogue (Variables|Default|GetNPCName) "Got that cookie yet?" (Utilities|Array|MakeArray "...not yet.")))
      (switch Utilities|FlowControl|Switch|SwitchonEnum_DialogueState _state_5
        (:NewEnumerator0
          (CallFunction|SetDialogueTreeIndex 2)
          (CallFunction|CloseConversation))))
    (:4
      (bind _state_6 (CallFunction|AddDialogue (Variables|Default|GetNPCName) "Cookie! Okay I'll open the door." (Utilities|Array|MakeArray "Thanks.")))
      (switch Utilities|FlowControl|Switch|SwitchonEnum_DialogueState _state_6
        (:NewEnumerator0
          (CallFunction|CloseConversation))))))