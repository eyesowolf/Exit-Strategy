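; Dialogue component for the Mum NPC, holding her party small talk and a fetch quest for a cookie in exchange for a funny Grandpa story.
; The Dialogue override calls its parent, then switches on DialogueTreeIndex to show lines and player options through AddDialogue.
; Branches update the index, then either loop back into the switch or close the conversation.
; A CheckPlayerItems test picks between the reminder and the story opening.
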(event EventBeginPlay)

(fn Dialogue
  (|CallParentFunction)
  (switch int (Variables|Default|GetDialogueTreeIndex) :!label _label
    (:0
      (bind (_state _optionindex) (CallFunction|AddDialogue (Variables|Default|GetNPCName) "Enjoying the party?" (Utilities|Array|MakeArray "It's great!" "About as much as I enjoy cream cheese on sushi.")))
      (switch Utilities|FlowControl|Switch|SwitchonEnum_DialogueState _state
        (:NewEnumerator0
          (switch int _optionindex
            (:0
              (bind _state_2 (CallFunction|AddDialogue (Variables|Default|GetNPCName) "Something tells me that's not entirely true." (Utilities|Array|MakeArray "...")))
              (switch Utilities|FlowControl|Switch|SwitchonEnum_DialogueState _state_2
                (:NewEnumerator0
                  (CallFunction|SetDialogueTreeIndex 1)
                  (goto _label))))
            (:1
              (bind _state_3 (CallFunction|AddDialogue (Variables|Default|GetNPCName) "Do you... like cream cheese on sushi?" (Utilities|Array|MakeArray "No.")))
              (switch Utilities|FlowControl|Switch|SwitchonEnum_DialogueState _state_3
                (:NewEnumerator0
                  (CallFunction|SetDialogueTreeIndex 1)
                  (goto _label))))))))
    (:1
      (bind (_state_4 _optionindex_2) (CallFunction|AddDialogue (Variables|Default|GetNPCName) "Want to know something funny?" (Utilities|Array|MakeArray "Yes. Please.")))
      (switch Utilities|FlowControl|Switch|SwitchonEnum_DialogueState _state_4
        (:NewEnumerator0
          (switch int _optionindex_2
            (:0
              (bind _state_5 (CallFunction|AddDialogue (Variables|Default|GetNPCName) "Get me a cookie from the snack table and I'll tell you." (Utilities|Array|MakeArray "Ugh fiiiine.")))
              (switch Utilities|FlowControl|Switch|SwitchonEnum_DialogueState _state_5
                (:NewEnumerator0
                  (CallFunction|SetDialogueTreeIndex 2)
                  (CallFunction|CloseConversation))))))))
    (:2
      (bind _hasitem (CallFunction|CheckPlayerItems "Cookie"))
      (if _hasitem
        (Variables|Default|SetDialogueTreeIndex 4)
        (goto _label)
        (else
          (CallFunction|SetDialogueTreeIndex 3)
          (goto _label))))
    (:3
      (bind _state_6 (CallFunction|AddDialogue (Variables|Default|GetNPCName) "Got that cookie yet?" (Utilities|Array|MakeArray "...not yet.")))
      (switch Utilities|FlowControl|Switch|SwitchonEnum_DialogueState _state_6
        (:NewEnumerator0
          (CallFunction|SetDialogueTreeIndex 2)
          (CallFunction|CloseConversation))))
    (:4
      (bind _state_7 (CallFunction|AddDialogue (Variables|Default|GetNPCName) "Cookie! Okay so, one time Grandpa - your Grandpa, as in my dad - not my Grandpa." (Utilities|Array|MakeArray "Yup I get it mum.")))
      (switch Utilities|FlowControl|Switch|SwitchonEnum_DialogueState _state_7
        (:NewEnumerator0
          (CallFunction|CloseConversation))))))