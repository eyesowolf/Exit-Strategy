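; Test dialogue component for an NPC that runs a two-step fetch quest, asking for a cube and then a sphere.
; The Dialogue override calls its parent, then switches on DialogueTreeIndex, looping back into the switch to chain states without closing the conversation.
; Player item checks choose between request and praise lines, each shown through AddDialogue.
; An unconnected branching small-talk graph never runs, and ConversationOpened is empty.
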(fn Dialogue
  (|CallParentFunction)
  (switch int (Variables|Default|GetDialogueTreeIndex) :!label _label
    (:0
      (bind _hasitem (CallFunction|CheckPlayerItems "Cube"))
      (if _hasitem
        (Variables|Default|SetDialogueTreeIndex 2)
        (goto _label)
        (else
          (CallFunction|SetDialogueTreeIndex 1)
          (goto _label))))
    (:1
      (bind _state (CallFunction|AddDialogue "NPC" "Could you get a cube for me?" (Utilities|Array|MakeArray "Of course!")))
      (switch Utilities|FlowControl|Switch|SwitchonEnum_DialogueState _state
        (:NewEnumerator0
          (CallFunction|SetDialogueTreeIndex)
          (CallFunction|CloseConversation))))
    (:2
      (bind _state_2 (CallFunction|AddDialogue "NPC" "What a nice cube!" (Utilities|Array|MakeArray "...")))
      (switch Utilities|FlowControl|Switch|SwitchonEnum_DialogueState _state_2
        (:NewEnumerator0
          (Variables|Default|SetDialogueTreeIndex 4)
          (goto _label))))
    (:3
      (bind _state_3 (CallFunction|AddDialogue "NPC" "Could you get a sphere for me next?" (Utilities|Array|MakeArray "No problem!")))
      (switch Utilities|FlowControl|Switch|SwitchonEnum_DialogueState _state_3
        (:NewEnumerator0
          (CallFunction|SetDialogueTreeIndex 4)
          (CallFunction|CloseConversation))))
    (:4
      (bind _hasitem_2 (CallFunction|CheckPlayerItems "Sphere"))
      (if _hasitem_2
        (Variables|Default|SetDialogueTreeIndex 5)
        (goto _label)
        (else
          (Variables|Default|SetDialogueTreeIndex 3)
          (goto _label))))
    (:5
      (bind _state_4 (CallFunction|AddDialogue "NPC" "What a nice sphere!" (Utilities|Array|MakeArray "...")))
      (switch Utilities|FlowControl|Switch|SwitchonEnum_DialogueState _state_4
        (:NewEnumerator0
          (CallFunction|CloseConversation))))))

(fn ConversationOpened
  (return 0))